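; BP_Character is a player-controlled character Blueprint with basic movement, jumping, a hold-to-speed-up key and simple health tracking.
; Move axes feed AddMovementInput along the control rotation's forward and right vectors, scaled by a Speed variable that rises while Tab is held.
; AnyDamage subtracts from Health and prints the result, with death only printing a "Dead" message.
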(event `InputAxis|MoveForward`
  (params (AxisValue :type "Float (single-precision)"))
  ;[1 1 1] 캐릭터 이동
  (`self.AddMovementInput` (`KismetMathLibrary.GetForwardVector` (`self.GetControlRotation`)) (* AxisValue (`self.Speed`))))

(event `InputAxis|MoveRight`
  (params (AxisValue :type "Float (single-precision)"))
  ;[1 1 1] 캐릭터 이동
  (`self.AddMovementInput` (`KismetMathLibrary.GetRightVector` (`self.GetControlRotation`)) (* AxisValue (`self.Speed`))))

(event `InputAction|Jump`
  (params (Key :type "Key Structure"))
  ;[1 1 1] 캐릭터 이동
  (:`Pressed`
    (`self.Jump`)))

(event `Key|Tab`
  (params (Key :type "Key Structure"))
  ;[1 1 1] 캐릭터 이동
  (:`Pressed`
    (set `self.Speed` 0.7))
  (:`Released`
    (set `self.Speed` 0.5)))

(event `self.ReceiveAnyDamage`
  (params (Damage :type "Float (single-precision)") (DamageType :type "DamageType Object Reference") (InstigatedBy :type "Controller Object Reference") (DamageCauser :type "Actor Object Reference"))
  (bind _output_get (set `self.Health` (- (`self.Health`) Damage)))
  (`KismetSystemLibrary.PrintString` (`KismetStringLibrary.Conv_DoubleToString` _output_get))
  (if (<= _output_get 0.0)
    (`KismetSystemLibrary.PrintString` "Dead")))

(fn `UserConstructionScript`)